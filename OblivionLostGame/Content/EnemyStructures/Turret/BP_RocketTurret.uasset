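; BP_RocketTurret is an enemy turret that aims and fires missiles at the player character when its PawnSensing component sees it.
; Each sighting yaws the Turret component toward the character, interpolating from the actor's rotation.
; It also restarts a retriggerable FireRate delay, so a shot follows only when no new sighting resets it.
; On completion it spawns a short-lived BP_Missile at the Arrow and plays a firing sound.
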(event `self.PawnSensing.OnSeePawn`
  (params (Pawn :type "Pawn Object Reference"))
  (bind _asbp_third_person_character (cast `/Game/ThirdPerson/Blueprints/BP_ThirdPersonCharacter` Pawn))
  (`|ExecutionSequence`
    (:`then_0`
      (bind (_returnvalue_roll _returnvalue_pitch _returnvalue_yaw) (`KismetMathLibrary.BreakRotator` (`KismetMathLibrary.RInterpTo` (`self.K2_GetActorRotation`) (`KismetMathLibrary.FindLookAtRotation` (`self.K2_GetActorLocation`) (`self.K2_GetActorLocation` _asbp_third_person_character)) (`GameplayStatics.GetWorldDeltaSeconds`) 500.0)))
      (`SceneComponent.K2_SetWorldRotation` (`self.Turret`) (`KismetMathLibrary.MakeRotator` 0.0 0.0 _returnvalue_yaw) false false))
    (:`then_1`
      (`KismetSystemLibrary.RetriggerableDelay` (`self.FireRate`))
      (bind _returnvalue (`|SpawnActorFromClass` "/Game/EnemyStructures/Turret/Missile/BP_Missile.BP_Missile_C" (`SceneComponent.K2_GetComponentToWorld` (`self.Arrow`)) "Undefined" "MultiplyWithRoot" null null))
      (`self.SetLifeSpan` _returnvalue 5.0)
      (`GameplayStatics.PlaySoundAtLocation` "/Game/Audio/SFX/Missile_Fire_War.Missile_Fire_War" (`self.K2_GetActorLocation`) (struct) 1.0 1.0 0.0 null null null null))))

(fn `UserConstructionScript`)