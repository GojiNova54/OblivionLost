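; BP_Missile is an explosive turret missile that homes in on player 0's capsule through its ProjectileMovement component.
; A blocking hit on anything but its owner spawns an explosion and sound, calls ApplyDamage and destroys the missile, while hitting the owner just destroys it.
; A separate Collision component hit event damages the player regardless of what was struck, and the actor-level ApplyDamage has no target wired.
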(event `self.ReceiveBeginPlay`
  (set `ProjectileMovementComponent.HomingTargetComponent` (`Character.CapsuleComponent` (`GameplayStatics.GetPlayerCharacter` 0)) (`self.ProjectileMovement`)))

(event `self.Collision.OnComponentHit`
  (params (HitComponent :type "PrimitiveComponent Object Reference") (OtherActor :type "Actor Object Reference") (OtherComp :type "PrimitiveComponent Object Reference") (NormalImpulse :type "Vector Structure") (Hit :type "HitResult Structure (by ref)"))
  (`GameplayStatics.ApplyDamage` (`GameplayStatics.GetPlayerCharacter` 0) (`self.Damage`)))

(event `self.ReceiveHit`
  (params (MyComp :type "PrimitiveComponent Object Reference") (Other :type "Actor Object Reference") (OtherComp :type "PrimitiveComponent Object Reference") (bSelfMoved :type Boolean) (HitLocation :type "Vector Structure") (HitNormal :type "Vector Structure") (NormalImpulse :type "Vector Structure") (Hit :type "HitResult Structure (by ref)"))
  (bind (_bblockinghit _binitialoverlap _time _distance _location _impactpoint _normal _impactnormal _physmat _hitactor) (`GameplayStatics.BreakHitResult` Hit))
  ;[1 0.6706 0.2488] On Hit
  (if _bblockinghit
    (if (!= _hitactor (`self.GetOwner`))
      (cast `Character` _hitactor
        (:`then`
          (`GameplayStatics.SpawnEmitterAtLocation` "/Game/StarterContent/Particles/P_Explosion.P_Explosion" _impactpoint (struct) (3.0 3.0 3.0))
          (`GameplayStatics.PlaySoundAtLocation` "/Game/StarterContent/Audio/Explosion02.Explosion02" _impactpoint (struct) 1.0 1.0 0.0 null null null null))
        (:`CastFailed`
          (`GameplayStatics.SpawnEmitterAtLocation` "/Game/StarterContent/Particles/P_Explosion.P_Explosion" _impactpoint (struct) (3.0 3.0 3.0))
          (`GameplayStatics.PlaySoundAtLocation` "/Game/StarterContent/Audio/Explosion02.Explosion02" _impactpoint (struct) 1.0 1.0 0.0 null null null null)))
      (`GameplayStatics.ApplyDamage` null (`self.Damage`) null (`self.GetOwner`))
      (`self.K2_DestroyActor`)
      (else
        (`self.K2_DestroyActor`)))))

(fn `UserConstructionScript`)